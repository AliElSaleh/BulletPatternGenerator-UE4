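; Base bullet pattern modifier for rotation rate, holding the state needed to alter how fast a spinnable pattern rotates.
; On Apply it runs the parent logic, casts the pattern to BulletPattern_SpinnableBase, then caches it and its starting rotation rate.
; Accessor functions expose the cached pattern, original rate and maximum rate.
; It never changes the rate itself, and patterns that fail the cast are not cached.
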(event `self.Apply`
  (params (InBulletPattern :type "BulletPattern_Base Object Reference"))
  (`parent.Apply` InBulletPattern)
  (bind _asbullet_pattern_spinnable_base (cast `BulletPattern_SpinnableBase` InBulletPattern))
  (bind _output_get (set `self.BulletPattern_Spinnable` _asbullet_pattern_spinnable_base))
  (`self.SetOriginalRotationRate` (`BulletPattern_SpinnableBase.RotationRate` _output_get)))

(fn `GetBulletPatternSpinnable`
  (returns (BulletPattern_Spinnable :type "BulletPattern_SpinnableBase Object Reference"))
  (return (`self.BulletPattern_Spinnable`)))

(fn `GetMaxRotationRate`
  (returns (`Return Value` :type "Rotator Structure"))
  (return (`self.MaxRotationRate`)))

(fn `GetOriginalRotationRate`
  (returns (`Return Value` :type "Rotator Structure"))
  (return (`self.OriginalRotationRate`)))

(fn `SetMaxRotationRate`
  (params (InMaxRotationRate :type "Rotator Structure"))
  (set `self.MaxRotationRate` InMaxRotationRate))

(fn `SetOriginalRotationRate`
  (params (InOriginalRotationRate :type "Rotator Structure"))
  (set `self.OriginalRotationRate` InOriginalRotationRate))