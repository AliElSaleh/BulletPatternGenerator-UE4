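; A showcase sine wave bullet pattern that alternates between fire and electric bullets by swapping its bullet pool at runtime.
; On each broadcast tick it runs the parent behavior and accumulates elapsed time, switching pools every couple of seconds.
; A class cast on the current pool decides which helper calls ChangeBulletPool with the other pool class.
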(event `self.Broadcast_Tick_Event`
  (params (DeltaTime :type "Float (single-precision)"))
  (`parent.Broadcast_Tick_Event` DeltaTime)
  (bind _output_get (set `self.TimeElapsed` (+ DeltaTime (`self.TimeElapsed`))))
  (if (> _output_get 2.0)
    (set `self.TimeElapsed` 0.0)
    (castclass `/Game/Blueprints/ObjectPools/BP_FireBulletPool` (`GameplayStatics.GetObjectClass` (`self.GetBulletPool`))
      (:`then`
        (`self.UseElectricBulletPool`))
      (:`CastFailed`
        (`self.UseFireBulletPool`)))))

(fn `UseElectricBulletPool`
  (`self.ChangeBulletPool` "/Game/Blueprints/ObjectPools/BP_ElectricBulletPool.BP_ElectricBulletPool_C"))

(fn `UseFireBulletPool`
  (`self.ChangeBulletPool` "/Game/Blueprints/ObjectPools/BP_FireBulletPool.BP_FireBulletPool_C"))