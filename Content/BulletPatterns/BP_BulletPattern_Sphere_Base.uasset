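; Sphere bullet pattern Blueprint that fires a bullet along each precomputed direction whenever the pattern updates.
; On begin play it stores the spawner's rotation and builds the direction list once via GenerateDirections.
; Directions are normalized offsets to points on a unit sphere around the spawner, stepping both angles together so they trace a single path rather than a full grid.
; The starting yaw is subtracted from phi without degree-to-radian conversion.
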(event `self.Broadcast_BeginPlay_Event`
  (`parent.Broadcast_BeginPlay_Event`)
  (`self.SetStartingRotation` (`Actor.K2_GetActorRotation` (`self.BulletPatternSpawner`)))
  (`self.GenerateDirections` 30))

(event `self.Broadcast_UpdatePattern_Event`
  (params (DeltaTime :type "Float (single-precision)"))
  (for _array_element (`self.Directions`)
    (`self.SpawnBulletInDirection` _array_element)))

(fn `GenerateDirections`
  (params (NumOfWays :type Integer))
  (bind (_startingrotation_roll _startingrotation_pitch _startingrotation_yaw) (`KismetMathLibrary.BreakRotator` (`self.StartingRotation`)))
  (bind _output_get (set `self.Angle` (/ 360.0 (`KismetMathLibrary.Conv_IntToDouble` NumOfWays))))
  (set `self.CurrentPhi` (`KismetMathLibrary.DegreesToRadians` _output_get))
  (`KismetArrayLibrary.Array_Clear` (`self.Directions`))
  (for _ (range (+ NumOfWays 1))
    (`KismetArrayLibrary.Array_Add` (`self.Directions`) (`KismetMathLibrary.Normal` (- (`BulletPatternFunctionLibrary.CalculateLocationOnSphere` (`Actor.K2_GetActorLocation` (`self.BulletPatternSpawner`)) 1.0 (`self.CurrentAngle`) (- (`self.CurrentPhi`) _startingrotation_yaw)) (`Actor.K2_GetActorLocation` (`self.BulletPatternSpawner`)))))
    (set `self.CurrentAngle` (+ (`self.CurrentAngle`) (`self.Angle`)))
    (set `self.CurrentPhi` (+ (`self.CurrentPhi`) (`KismetMathLibrary.DegreesToRadians` (`self.Angle`))))))