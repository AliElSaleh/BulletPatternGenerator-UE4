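; Base bullet pattern modifier that gradually raises a pattern's fire rate after it is applied.
; On Apply it caches the pattern's original fire rate and derives a maximum by adding a configurable increase amount.
; Each tick it maps elapsed time over a fixed three-second window to a clamped linear ramp between those rates and writes the result back to the pattern.
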(event `self.Apply`
  (params (InBulletPattern :type "BulletPattern_Base Object Reference"))
  (`parent.Apply` InBulletPattern)
  (bind _output_get (set `self.OriginalFireRate` (`BulletPattern_Base.GetFireRate` InBulletPattern)))
  (set `self.MaxFireRate` (+ _output_get (`self.FireRateIncreaseAmount`))))

(event `self.Tick`
  (params (DeltaTime :type "Float (single-precision)"))
  (`parent.Tick` DeltaTime)
  (`BulletPattern_Base.SetFireRate` (`self.BulletPattern`) (`KismetMathLibrary.MapRangeClamped` (`self.ElapsedTime`) 0.0 3.0 (`self.OriginalFireRate`) (`self.MaxFireRate`))))