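; Bullet pattern modifier that periodically switches the pattern's bullet pool, named for toggling between fire and electric bullets.
; On apply it calls the parent, then starts a looping timer at the ToggleEvery interval.
; Each tick it sets the pattern to the next entry in BulletPoolsToCycle, wrapping back to the first after the last.
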(event `self.OnModifierApplied`
  (`parent.OnModifierApplied`)
  (`KismetSystemLibrary.K2_SetTimerDelegate` (delegate `CustomEvent_0`) (`self.ToggleEvery`) true))

(event `CustomEvent_0`
  (if (> (`self.Index`) (- (`KismetArrayLibrary.Array_Length` (`self.BulletPoolsToCycle`)) 1))
    (set `self.Index` 0))
  (`BulletPattern_Base.ChangeBulletPool` (`self.BulletPattern`) (`|GetArrayItem` (`self.BulletPoolsToCycle`) (`self.Index`)))
  (`/Engine/EditorBlueprintResources/StandardMacros.IncrementInt` (`self.Index`)))