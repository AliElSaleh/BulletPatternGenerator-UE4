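; Linear bullet pattern Blueprint, currently a stub with no working behavior.
; BeginPlay, Tick, EndPlay and the UpdatePattern event all have empty bodies.
; The only other nodes are disconnected debug leftovers that print messages, clear a Hello flag and accumulate an Uptime counter, none of which ever run.
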(event `self.ReceiveBeginPlay`)

(event `self.ReceiveTick`
  (params (DeltaTime :type "Float (single-precision)")))

(event `self.ReceiveEndPlay`
  (params (EndPlayReason :type "EEndPlayReason Enum" :default "Destroyed")))

(event `self.ReceiveUpdatePattern`
  (params (DeltaTime :type "Float (single-precision)")))