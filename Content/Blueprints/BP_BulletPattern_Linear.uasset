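; BP_BulletPattern_Linear is a Blueprint named for a linear bullet pattern, but it contains only lifecycle debug logging and no bullet logic.
; BeginPlay prints a greeting, clears the Hello flag and prints its value.
; Tick accumulates delta time into Uptime and prints it every frame.
; EndPlay prints a farewell and the current Hello value.
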(event `self.ReceiveBeginPlay`
  (`KismetSystemLibrary.PrintString` null "Hello Begin Play")
  (bind _output_get (set `self.bHello` false))
  (`KismetSystemLibrary.PrintString` null (`KismetStringLibrary.Conv_BoolToString` _output_get)))

(event `self.ReceiveTick`
  (params (DeltaTime :type "Float (single-precision)"))
  (bind _output_get (set `self.Uptime` (+ DeltaTime (`self.Uptime`))))
  (`KismetSystemLibrary.PrintString` null (`KismetStringLibrary.Concat_StrStr` (`KismetStringLibrary.Conv_DoubleToString` _output_get) ": Hello Tick")))

(event `self.ReceiveEndPlay`
  (params (EndPlayReason :type "EEndPlayReason Enum" :default "Destroyed"))
  (`KismetSystemLibrary.PrintString` null "Hello End Play")
  (`KismetSystemLibrary.PrintString` null (`KismetStringLibrary.Conv_BoolToString` (`self.bHello`))))