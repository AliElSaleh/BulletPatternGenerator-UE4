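; Bullet pattern that fires a ring of bullets, nominally 40-way going by its name, from its spawner.
; On begin play it takes the spawner's rotation and precomputes normalized directions, stepping 360/NumOfWays around a unit sphere with starting yaw as phi.
; Each pattern update spawns a bullet along every cached direction, so the ring does not follow later spawner rotation.
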(event `self.Broadcast_BeginPlay_Event`
  (`parent.Broadcast_BeginPlay_Event`)
  (`self.SetStartingRotation` (`Actor.K2_GetActorRotation` (`self.BulletPatternSpawner`)))
  (`self.GenerateBulletDirections` (`self.NumOfWays`)))

(event `self.Broadcast_UpdatePattern_Event`
  (params (DeltaTime :type "Float (single-precision)"))
  (for _array_element (`self.Directions`)
    (`self.SpawnBulletInDirection` _array_element)))

(fn `GenerateBulletDirections`
  (params (InNumOfWays :type Integer))
  (locals (CurrentAngle :type "Float (double-precision)"))
  (bind (_startingrotation_roll _startingrotation_pitch _startingrotation_yaw) (`KismetMathLibrary.BreakRotator` (`self.StartingRotation`)))
  (set `self.Angle` (/ 360.0 (`KismetMathLibrary.Conv_IntToDouble` InNumOfWays)))
  (`KismetArrayLibrary.Array_Clear` (`self.Directions`))
  (for _ (range (+ InNumOfWays 1))
    (`KismetArrayLibrary.Array_Add` (`self.Directions`) (`KismetMathLibrary.Normal` (- (`BulletPatternFunctionLibrary.CalculateLocationOnSphere` (`Actor.K2_GetActorLocation` (`self.BulletPatternSpawner`)) 1.0 (`local.CurrentAngle`) (`KismetMathLibrary.DegreesToRadians` _startingrotation_yaw)) (`Actor.K2_GetActorLocation` (`self.BulletPatternSpawner`)))))
    (set `local.CurrentAngle` (+ (`local.CurrentAngle`) (`self.Angle`)))))