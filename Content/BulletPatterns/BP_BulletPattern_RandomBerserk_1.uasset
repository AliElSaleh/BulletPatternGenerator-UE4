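; BP_BulletPattern_RandomBerserk_1 is a bullet pattern that fires a burst of bullets in random directions.
; On begin play it fills Directions with random unit vectors, using a random way count from 3 to 25.
; Tick regenerates that set once elapsed time passes a random threshold, re-rolled every frame.
; Each pattern update spawns a bullet along every stored direction; the computed Angle spacing is unused.
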(event `self.Broadcast_BeginPlay_Event`
  (`parent.Broadcast_BeginPlay_Event`)
  (`self.GenerateBulletDirections` (`KismetMathLibrary.RandomIntegerInRange` 3 25)))

(event `self.Broadcast_Tick_Event`
  (params (DeltaTime :type "Float (single-precision)"))
  (`parent.Broadcast_Tick_Event` DeltaTime)
  (bind _output_get (set `self.ElapsedTime` (+ DeltaTime (`self.ElapsedTime`))))
  (if (> _output_get (`KismetMathLibrary.RandomFloatInRange` 0.5 2.0))
    (set `self.ElapsedTime` 0.0)
    (`self.GenerateBulletDirections` (`KismetMathLibrary.RandomIntegerInRange` 3 25))))

(event `self.Broadcast_UpdatePattern_Event`
  (params (DeltaTime :type "Float (single-precision)"))
  (for _array_element (`self.Directions`)
    (`self.SpawnBulletInDirection` _array_element)))

(fn `GenerateBulletDirections`
  (params (InNumOfWays :type Integer))
  (set `self.Angle` (/ 360.0 (`KismetMathLibrary.Conv_IntToDouble` InNumOfWays)))
  (`KismetArrayLibrary.Array_Clear` (`self.Directions`))
  (for _ (range (+ InNumOfWays 1))
    (`KismetArrayLibrary.Array_Add` (`self.Directions`) (`KismetMathLibrary.RandomUnitVector`))))