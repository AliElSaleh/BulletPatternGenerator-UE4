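; Bullet pattern that builds firing directions for an all-round spherical burst around its spawner.
; GenerateDirections uses nested loops over latitude-like rings and evenly stepped angles, both derived from NumOfWays.
; Each sample is a unit-sphere point from CalculateLocationOnSphere, converted to a normalized direction from the spawner and stored in Directions.
; The resulting direction count is printed for debugging.
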(fn `GenerateDirections`
  (params (NumOfWays :type Integer))
  (set `self.Angle` (/ 360.0 (`KismetMathLibrary.Conv_IntToDouble` NumOfWays)))
  (set `self.CurrentPhi` 0.0)
  (`KismetArrayLibrary.Array_Clear` (`self.Directions`))
  (for _ (range (+ (/ NumOfWays 2) 1))
    (for _ (range NumOfWays)
      (`KismetArrayLibrary.Array_Add` (`self.Directions`) (`KismetMathLibrary.Normal` (- (`BulletPatternFunctionLibrary.CalculateLocationOnSphere` (`Actor.K2_GetActorLocation` (`self.BulletPatternSpawner`)) 1.0 (`self.CurrentAngle`) (`self.CurrentPhi`)) (`Actor.K2_GetActorLocation` (`self.BulletPatternSpawner`)))))
      (set `self.CurrentAngle` (+ (`self.CurrentAngle`) (`self.Angle`))))
    (set `self.CurrentPhi` (+ (`self.CurrentPhi`) (`KismetMathLibrary.DegreesToRadians` (/ (/ 360.0 (`KismetMathLibrary.Conv_IntToDouble` (/ NumOfWays 2))) 2.0))))
    (set `self.CurrentAngle` (/ 360.0 (`KismetMathLibrary.Conv_IntToDouble` NumOfWays))))
  (`KismetSystemLibrary.PrintString` null (`KismetStringLibrary.Conv_IntToString` (`KismetArrayLibrary.Array_Length` (`self.Directions`)))))