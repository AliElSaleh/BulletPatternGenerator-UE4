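; Bullet pattern modifier that ping-pongs the pattern's bullet speed between its original and maximum values.
; Tick uses clamped range mapping on ElapsedTime to ramp speed up over the first second and back down over the next, then resets the timer to loop.
; Apply only calls the parent, and the speed limits come from getters not defined in this graph.
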(event `self.Tick`
  (params (DeltaTime :type "Float (single-precision)"))
  (bind _elapsedtime (`self.ElapsedTime`))
  (`parent.Tick` DeltaTime)
  (if (> _elapsedtime 1.0)
    (`BulletPattern_Base.SetBulletSpeed` (`self.BulletPattern`) (`KismetMathLibrary.MapRangeClamped` _elapsedtime 1.0 2.0 (`self.GetMaxBulletSpeed`) (`self.GetOriginalBulletSpeed`)))
    (if (> _elapsedtime 2.0)
      (set `self.ElapsedTime` 0.0))
    (else
      (`BulletPattern_Base.SetBulletSpeed` (`self.BulletPattern`) (`KismetMathLibrary.MapRangeClamped` _elapsedtime 0.0 1.0 (`self.GetOriginalBulletSpeed`) (`self.GetMaxBulletSpeed`))))))

(event `self.Apply`
  (params (InBulletPattern :type "BulletPattern_Base Object Reference"))
  (`parent.Apply` InBulletPattern))