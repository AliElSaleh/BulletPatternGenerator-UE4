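; Bullet pattern Blueprint that locks a linear shot onto the player.
; On each broadcast tick event it computes the direction from the spawner to the player as a rotation.
; It stores that rotation's forward vector as the bullet direction and rotates the spawner actor to face the player.
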(event `self.Broadcast_Tick_Event`
  (params (DeltaTime :type "Float (single-precision)"))
  (bind _output_get (set `self.TargetRotation` (`KismetMathLibrary.Conv_VectorToRotator` (- (`Actor.K2_GetActorLocation` (`self.Player`)) (`Actor.K2_GetActorLocation` (`self.BulletPatternSpawner`))))))
  (set `self.BulletDirection` (`KismetMathLibrary.Conv_RotatorToVector` _output_get))
  (`Actor.K2_SetActorRotation` (`self.BulletPatternSpawner`) _output_get false))