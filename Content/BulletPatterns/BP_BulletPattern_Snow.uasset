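; Snow bullet pattern that builds a cloud of still bullets around its spawner, then releases them together.
; Each pattern update spawns a zero-direction bullet and moves it to a random point on a sphere of SpawnRadius.
; After three seconds, tick halts spawning, sends every bullet along one shared fixed direction at random one to two times base speed, and stops the spawner's pattern.
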(event `self.Broadcast_BeginPlay_Event`
  (`parent.Broadcast_BeginPlay_Event`)
  (set `self.bSpawnBullets` true))

(event `self.Broadcast_UpdatePattern_Event`
  (params (DeltaTime :type "Float (single-precision)"))
  (if (`self.bSpawnBullets`)
    (bind _output_get (set `self.Counter` (+ (`self.Counter`) 1)))
    (`KismetArrayLibrary.Array_Add` (`self.Indices`) _output_get)
    (bind _returnvalue (`self.SpawnBulletInDirection` (`KismetMathLibrary.MakeVector` 0.0)))
    (`Actor.K2_SetActorLocation` _returnvalue (`BulletPatternFunctionLibrary.CalculateLocationOnSphere` (`Actor.K2_GetActorLocation` (`self.BulletPatternSpawner`)) (`self.SpawnRadius`) (`KismetMathLibrary.RandomFloatInRange` 0.0 360.0) (`KismetMathLibrary.RandomFloatInRange` 0.0 6.28318)) false false)))

(event `self.Broadcast_Tick_Event`
  (params (DeltaTime :type "Float (single-precision)"))
  (bind _returnvalue (`self.GetBulletSpeed`))
  (`parent.Broadcast_Tick_Event` DeltaTime)
  (if (> (`self.ElapsedTime`) 3.0)
    (set `self.bSpawnBullets` false)
    (for _array_element (`self.Bullets`)
      (`Bullet.SetupBehaviour` _array_element self (`KismetMathLibrary.GetUpVector` (struct :`Pitch` 180.0)) (`KismetMathLibrary.RandomFloatInRange` _returnvalue (* _returnvalue 2.0))))
    (`BulletPatternSpawner.StopBulletPattern` (`self.BulletPatternSpawner`))))