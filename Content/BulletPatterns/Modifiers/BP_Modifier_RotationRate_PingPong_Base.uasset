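; Bullet-pattern modifier base that ping-pongs a spinnable pattern's rotation rate between its original and max rates.
; Each Tick runs the parent tick, then linearly maps elapsed time per axis, ramping up over MaxTime and back down over GracePeriod.
; Once elapsed time passes the combined span, it resets to zero so the cycle repeats.
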(event `self.Tick`
  (params (DeltaTime :type "Float (single-precision)"))
  (bind (_return_value_roll _return_value_pitch _return_value_yaw) (`KismetMathLibrary.BreakRotator` (`self.GetMaxRotationRate`)))
  (bind (_return_value_roll_2 _return_value_pitch_2 _return_value_yaw_2) (`KismetMathLibrary.BreakRotator` (`self.GetOriginalRotationRate`)))
  (bind (_return_value_roll_3 _return_value_pitch_3 _return_value_yaw_3) (`KismetMathLibrary.BreakRotator` (`self.GetMaxRotationRate`)))
  (bind (_return_value_roll_4 _return_value_pitch_4 _return_value_yaw_4) (`KismetMathLibrary.BreakRotator` (`self.GetOriginalRotationRate`)))
  (bind _maxtime (`self.MaxTime`))
  (bind _maxtime_2 (`self.MaxTime`))
  (bind _maxtime_3 (`self.MaxTime`))
  (`parent.Tick` DeltaTime)
  (if (> (`self.ElapsedTime`) (`self.MaxTime`))
    (set `BulletPattern_SpinnableBase.RotationRate` (`KismetMathLibrary.MakeRotator` (`KismetMathLibrary.MapRangeClamped` (`self.ElapsedTime`) _maxtime_2 (+ _maxtime_2 (`self.GracePeriod`)) _return_value_roll _return_value_roll_4) (`KismetMathLibrary.MapRangeClamped` (`self.ElapsedTime`) _maxtime (+ _maxtime (`self.GracePeriod`)) _return_value_pitch _return_value_pitch_4) (`KismetMathLibrary.MapRangeClamped` (`self.ElapsedTime`) _maxtime_3 (+ _maxtime_3 (`self.GracePeriod`)) _return_value_yaw _return_value_yaw_4)) (`self.GetBulletPatternSpinnable`))
    (if (> (`self.ElapsedTime`) (+ (`self.MaxTime`) (`self.GracePeriod`)))
      (set `self.ElapsedTime` 0.0))
    (else
      (set `BulletPattern_SpinnableBase.RotationRate` (`KismetMathLibrary.MakeRotator` (`KismetMathLibrary.MapRangeClamped` (`self.ElapsedTime`) 0.0 (`self.MaxTime`) _return_value_roll_2 _return_value_roll_3) (`KismetMathLibrary.MapRangeClamped` (`self.ElapsedTime`) 0.0 (`self.MaxTime`) _return_value_pitch_2 _return_value_pitch_3) (`KismetMathLibrary.MapRangeClamped` (`self.ElapsedTime`) 0.0 (`self.MaxTime`) _return_value_yaw_2 _return_value_yaw_3)) (`self.GetBulletPatternSpinnable`)))))