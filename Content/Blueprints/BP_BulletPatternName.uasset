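; BP_BulletPatternName labels a bullet pattern spawner by showing the name of its active pattern on a text render component.
; The construction script reads PatternName from the class defaults of the spawner's active pattern, so no pattern instance is needed.
; An optional character index splits the name with an inserted line-break tag.
; Refresh resets to false whenever the script runs with a valid spawner, acting as an editor update toggle.
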(fn `UserConstructionScript`
  (bind _textchararray (`self.TextCharArray`))
  (bind _insertnewlineatindex (`self.InsertNewLineAtIndex`))
  (bind _insertnewlineatindex_2 (`self.InsertNewLineAtIndex`))
  (`/Engine/EditorBlueprintResources/StandardMacros.IsValid` (`self.BulletPatternSpawner`)
    (:`Is Valid`
      (set `self.bRefresh` false)
      (bind _output_get (set `self.RawPatternName` (`KismetStringLibrary.Conv_NameToString` (defaults `/Game/Blueprints/BP_BulletPatternName` (`BulletPatternSpawner.GetActiveBulletPatternClass` (`self.BulletPatternSpawner`))))))
      (set `self.TextCharArray` (`KismetStringLibrary.GetCharacterArrayFromString` _output_get))
      (if (or (>= _insertnewlineatindex_2 (`KismetArrayLibrary.Array_Length` (`self.TextCharArray`))) (== _insertnewlineatindex_2 0))
        (`TextRenderComponent.K2_SetText` (`self.TextRender`) (`KismetTextLibrary.Conv_StringToText` (`self.RawPatternName`)))
        (else
          (for (_ _array_index) (`self.TextCharArray`)
            (if (and (== _array_index _insertnewlineatindex) (!= _insertnewlineatindex 0))
              (`KismetArrayLibrary.Array_Insert` _textchararray "<br>" _array_index)
              (`TextRenderComponent.K2_SetText` (`self.TextRender`) (`KismetTextLibrary.Conv_StringToText` (`KismetStringLibrary.JoinStringArray` _textchararray "")))
              (break))))))))