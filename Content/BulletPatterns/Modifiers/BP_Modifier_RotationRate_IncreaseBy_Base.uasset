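; Base bullet pattern modifier that gradually changes the rotation rate of a spinnable bullet pattern.
; Each Tick, after the parent Tick, it adds RotationRateIncrementAmount to the pattern's RotationRate per axis.
; Roll, pitch and yaw are each clamped between the original and maximum rotation rates.
; The increment is not scaled by DeltaTime, so the ramp speed depends on tick frequency.
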(event `self.Tick`
  (params (DeltaTime :type "Float (single-precision)"))
  (bind (_return_value_roll _return_value_pitch _return_value_yaw) (`KismetMathLibrary.BreakRotator` (`self.GetMaxRotationRate`)))
  (bind (_return_value_roll_2 _return_value_pitch_2 _return_value_yaw_2) (`KismetMathLibrary.BreakRotator` (`self.GetOriginalRotationRate`)))
  (bind (_rotationrateincrementamount_roll _rotationrateincrementamount_pitch _rotationrateincrementamount_yaw) (`KismetMathLibrary.BreakRotator` (`self.RotationRateIncrementAmount`)))
  (bind (_rotationrate_roll _rotationrate_pitch _rotationrate_yaw) (`KismetMathLibrary.BreakRotator` (`BulletPattern_SpinnableBase.RotationRate` (`self.GetBulletPatternSpinnable`))))
  (`parent.Tick` DeltaTime)
  (set `BulletPattern_SpinnableBase.RotationRate` (`KismetMathLibrary.MakeRotator` (`KismetMathLibrary.FClamp` (+ _rotationrate_roll _rotationrateincrementamount_roll) _return_value_roll_2 _return_value_roll) (`KismetMathLibrary.FClamp` (+ _rotationrate_pitch _rotationrateincrementamount_pitch) _return_value_pitch_2 _return_value_pitch) (`KismetMathLibrary.FClamp` (+ _rotationrate_yaw _rotationrateincrementamount_yaw) _return_value_yaw_2 _return_value_yaw)) (`self.GetBulletPatternSpinnable`)))