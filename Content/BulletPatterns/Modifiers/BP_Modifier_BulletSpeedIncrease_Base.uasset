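; Base bullet pattern modifier that ramps up a pattern's bullet speed over time.
; On Apply it records the pattern's original speed and computes a maximum by adding the configured increase amount.
; Each Tick it maps elapsed time with a clamped range, raising speed linearly to that maximum over the first three seconds.
; Getters expose the original speed, maximum speed and increase amount.
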(event `self.Apply`
  (params (InBulletPattern :type "BulletPattern_Base Object Reference"))
  (`parent.Apply` InBulletPattern)
  (bind _output_get (set `self.OriginalBulletSpeed` (`BulletPattern_Base.GetBulletSpeed` InBulletPattern)))
  (set `self.MaxBulletSpeed` (+ _output_get (`self.SpeedIncreaseAmount`))))

(event `self.Tick`
  (params (DeltaTime :type "Float (single-precision)"))
  (`parent.Tick` DeltaTime)
  (`BulletPattern_Base.SetBulletSpeed` (`self.BulletPattern`) (`KismetMathLibrary.MapRangeClamped` (`self.ElapsedTime`) 0.0 3.0 (`self.OriginalBulletSpeed`) (`self.MaxBulletSpeed`))))

(fn `GetMaxBulletSpeed`
  (returns (`Return Value` :type "Float (double-precision)"))
  (return (`self.MaxBulletSpeed`)))

(fn `GetOriginalBulletSpeed`
  (returns (`Return Value` :type "Float (double-precision)"))
  (return (`self.OriginalBulletSpeed`)))

(fn `GetSpeedIncreaseAmount`
  (returns (`Return Value` :type "Float (double-precision)"))
  (return (`self.SpeedIncreaseAmount`)))