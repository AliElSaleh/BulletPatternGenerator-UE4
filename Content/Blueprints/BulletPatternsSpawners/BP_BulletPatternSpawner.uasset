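; Spawner actor that fires pooled bullets in a spinning pattern for bullet-pattern gameplay.
; On BeginPlay it gets the "Fire Bullets" object pool, then after a short delay starts its configured pattern, which sets a looping fire timer and the RotatingMovement spin.
; SpawnBullet launches a pooled bullet along the actor's forward vector at the pattern's speed.
; ChangeBulletPattern can swap patterns, but its test timer and the non-pooled spawn code are disconnected.
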(event `self.ReceiveBeginPlay`
  (bind _asbp_fire_bullet_pool (cast `/Game/Blueprints/ObjectPools/BP_FireBulletPool` (`ObjectPoolFunctionLibrary.GetObjectPool` self "Fire Bullets")))
  (set `self.FireBulletPool` _asbp_fire_bullet_pool)
  (`KismetSystemLibrary.Delay` 1.0)
  (`self.StartBulletPattern` (`self.BulletPattern`)))

(event `UpdatePattern`
  (`self.ChangeBulletPattern` null))

(fn `ChangeBulletPattern`
  (params (NewBulletPattern :type "BulletPatternBase Object Reference"))
  (`self.StopBulletPattern`)
  (bind _output_get (set `self.ActiveBulletPattern` NewBulletPattern))
  (`self.StartBulletPattern` _output_get))

(fn `SpawnBullet`
  (bind _returnvalue (`ObjectPoolBase.GetActorFromPool` (`self.FireBulletPool`)))
  (`/Engine/EditorBlueprintResources/StandardMacros.IsValid` _returnvalue
    (:`Is Valid`
      (bind _asbp_bullet_base (cast `/Game/Blueprints/Bullets/BP_BulletBase` _returnvalue))
      (`self.K2_SetActorLocation` _asbp_bullet_base (`self.K2_GetActorLocation`) false true)
      (`Bullet.SetupBehaviour` _asbp_bullet_base null (`self.GetActorForwardVector`) (`BulletPatternBase.BulletSpeed` (`self.ActiveBulletPattern`)))
      (`PooledActor.PooledActor_BeginPlay` _asbp_bullet_base))))

(fn `StartBulletPattern`
  (params (BulletPattern :type "BulletPatternBase Object Reference"))
  (set `self.ActiveBulletPattern` BulletPattern)
  (bind _returnvalue (`KismetSystemLibrary.K2_SetTimerDelegate` (`|CreateDelegate` self :!event `SpawnBullet`) (`BulletPatternBase.FireRate` BulletPattern) true))
  (set `self.BulletSpawnerTimer` _returnvalue)
  (set `RotatingMovementComponent.RotationRate` (`KismetMathLibrary.MakeRotator` 0.0 0.0 (`BulletPatternBase.SpinSpeed` BulletPattern)) (`self.RotatingMovement`)))

(fn `StopBulletPattern`
  (`KismetSystemLibrary.K2_ClearAndInvalidateTimerHandle` (`self.BulletSpawnerTimer`)))

(fn `UserConstructionScript`)