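; Bullet pattern that fires a radial set of bullets from a continuously rotating spawner, named Twisting StarFish.
; Each tick advances the starting rotation by RotationRate and applies it to the spawner actor.
; Each pattern update rebuilds evenly stepped directions on a sphere, using yaw as phi and an accumulating angle, then spawns bullets along them.
; Modifier 0 applies at begin play; modifiers 1 to 3 apply every tick after two seconds.
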(event `self.Broadcast_BeginPlay_Event`
  (`parent.Broadcast_BeginPlay_Event`)
  (`self.SetStartingRotation` (`Actor.K2_GetActorRotation` (`self.BulletPatternSpawner`)))
  (`self.GenerateBulletDirections` (`self.NumOfWays`))
  (`self.ApplyModifier` 0))

(event `self.Broadcast_Tick_Event`
  (params (DeltaTime :type "Float (single-precision)"))
  (bind (_rotationrate_roll _rotationrate_pitch _rotationrate_yaw) (`KismetMathLibrary.BreakRotator` (`self.RotationRate`)))
  (bind (_startingrotation_roll _startingrotation_pitch _startingrotation_yaw) (`KismetMathLibrary.BreakRotator` (`self.StartingRotation`)))
  (`parent.Broadcast_Tick_Event` DeltaTime)
  (`self.SetStartingRotation` (`KismetMathLibrary.MakeRotator` (+ (* _rotationrate_roll DeltaTime) _startingrotation_roll) (+ (* _rotationrate_pitch DeltaTime) _startingrotation_pitch) (+ (* _rotationrate_yaw DeltaTime) _startingrotation_yaw)))
  (`Actor.K2_SetActorRotation` (`self.BulletPatternSpawner`) (`self.StartingRotation`) false)
  (if (> (`self.ElapsedTime`) 2.0)
    (`self.ApplyModifier` 1)
    (`self.ApplyModifier` 2)
    (`self.ApplyModifier` 3)))

(event `self.Broadcast_UpdatePattern_Event`
  (params (DeltaTime :type "Float (single-precision)"))
  (`self.GenerateBulletDirections` (`self.NumOfWays`))
  (for _array_element (`self.Directions`)
    (`self.SpawnBulletInDirection` _array_element)))

(fn `GenerateBulletDirections`
  (params (InNumOfWays :type Integer))
  (locals (CurrentAngle :type "Float (double-precision)"))
  (bind (_startingrotation_roll _startingrotation_pitch _startingrotation_yaw) (`KismetMathLibrary.BreakRotator` (`self.StartingRotation`)))
  (set `self.Angle` (/ 360.0 (`KismetMathLibrary.Conv_IntToDouble` InNumOfWays)))
  (`KismetArrayLibrary.Array_Clear` (`self.Directions`))
  (for _ (range (+ InNumOfWays 1))
    (`KismetArrayLibrary.Array_Add` (`self.Directions`) (`KismetMathLibrary.Normal` (- (`BulletPatternFunctionLibrary.CalculateLocationOnSphere` (`Actor.K2_GetActorLocation` (`self.BulletPatternSpawner`)) 1.0 (`local.CurrentAngle`) (`KismetMathLibrary.DegreesToRadians` _startingrotation_yaw)) (`Actor.K2_GetActorLocation` (`self.BulletPatternSpawner`)))))
    (set `local.CurrentAngle` (+ (`local.CurrentAngle`) (`self.Angle`)))))